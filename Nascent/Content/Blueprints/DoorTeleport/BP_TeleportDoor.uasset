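; BP_TeleportDoor is a numbered door that moves the player to a set location when overlapped with a matching KeysCollected count.
; The box overlap casts to BP_BaseCharacter and requires KeysCollected to equal DoorNumber exactly before setting the actor location.
; From BeginPlay, a delayed polling loop checks the player's count, showing BasicAsset02 on the cube until it matches, then switching to BackgroundMaterial and ending.
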(event `Check For Color Update`
  (bind _cube (`self.Cube`))
  (bind _asbp_base_character (cast `/Game/Blueprints/Player_Blueprints/BP_BaseCharacter` (`GameplayStatics.GetPlayerPawn` 0)))
  (if (== (`/Game/Blueprints/Player_Blueprints/BP_BaseCharacter.Keys Collected` _asbp_base_character) (`self.Door number`)) :!label _label
    (`PrimitiveComponent.SetMaterial` _cube 0 "/Engine/EngineMeshes/BackgroundMaterial.BackgroundMaterial")
    (elif (not (== (`MeshComponent.OverlayMaterial` _cube) "/Engine/MapTemplates/Materials/BasicAsset02.BasicAsset02"))
      (`PrimitiveComponent.SetMaterial` _cube 0 "/Engine/MapTemplates/Materials/BasicAsset02.BasicAsset02")
      (`KismetSystemLibrary.Delay` 1.0)
      (goto _label))))

(event `self.ReceiveBeginPlay`
  (`self.Check For Color Update`))

(event `self.Box.OnComponentBeginOverlap`
  (params (OverlappedComponent :type "PrimitiveComponent Object Reference") (OtherActor :type "Actor Object Reference") (OtherComp :type "PrimitiveComponent Object Reference") (OtherBodyIndex :type Integer) (bFromSweep :type Boolean) (SweepResult :type "HitResult Structure (by ref)"))
  (bind _asbp_base_character (cast `/Game/Blueprints/Player_Blueprints/BP_BaseCharacter` OtherActor)
    (:`then`
      (if (== (`/Game/Blueprints/Player_Blueprints/BP_BaseCharacter.Keys Collected` _asbp_base_character) (`self.Door number`))
        (`self.K2_SetActorLocation` _asbp_base_character (`self.Teleport Location`) false false)))
    (:`CastFailed`
      (`KismetSystemLibrary.PrintString` "Cast Failed"))))

(fn `UserConstructionScript`)