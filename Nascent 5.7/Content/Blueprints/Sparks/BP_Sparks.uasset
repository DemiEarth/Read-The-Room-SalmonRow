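; BP_Sparks is a spark actor meant to be pulled toward a BP_BaseCharacter and then disappear.
; Entering SphereCollision fires PullToTarget once, applying a single delta-time-scaled local offset along the character's normalized world position, not the vector from spark to character.
; A character hit on the Sphere mesh prints a debug string and destroys the actor after a short delay.
; BeginPlay applies SparkMaterial to the Sphere.
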(event `self.ReceiveBeginPlay`
  (`PrimitiveComponent.SetMaterial` (`self.Sphere`) 0 (`self.Spark Material`)))

(event `self.Sphere collision.OnComponentBeginOverlap`
  (params (OverlappedComponent :type "PrimitiveComponent Object Reference") (OtherActor :type "Actor Object Reference") (OtherComp :type "PrimitiveComponent Object Reference") (OtherBodyIndex :type Integer) (bFromSweep :type Boolean) (SweepResult :type "HitResult Structure (by ref)"))
  (bind _asbp_base_character (cast `/Game/Blueprints/Player_Blueprints/BP_BaseCharacter` OtherActor))
  (`self.pull to target` _asbp_base_character))

(event `self.Sphere.OnComponentHit`
  (params (HitComponent :type "PrimitiveComponent Object Reference") (OtherActor :type "Actor Object Reference") (OtherComp :type "PrimitiveComponent Object Reference") (NormalImpulse :type "Vector Structure") (Hit :type "HitResult Structure (by ref)"))
  (cast `/Game/Blueprints/Player_Blueprints/BP_BaseCharacter` OtherActor)
  (`KismetSystemLibrary.PrintString` "Pulled")
  (`KismetSystemLibrary.Delay` 0.2)
  (`self.K2_DestroyActor`))

(event `pull to target`
  (params (Target :type "Actor Object Reference"))
  (`self.K2_AddActorLocalOffset` (* (`KismetMathLibrary.Normal` (- (`self.K2_GetActorLocation` Target) (0.0 0.0 0.0))) (`GameplayStatics.GetWorldDeltaSeconds`) (`self.Speed`))))

(fn `UserConstructionScript`)