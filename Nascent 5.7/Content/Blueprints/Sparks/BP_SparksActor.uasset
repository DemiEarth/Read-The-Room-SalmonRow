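; Collectible spark actor that raises the player's spark count and can unlock movement abilities.
; On overlap with a BP_BaseCharacter, it increments the count, waits briefly, calls DestroyActor, then runs UnlockMechanic.
; UnlockMechanic uses per-spark flags to enable grapple or climb, or increase jump count, on player pawn 0.
; BeginPlay applies the spark material and records the sphere's starting location, which this graph never reads.
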(event `self.ReceiveBeginPlay`
  (`PrimitiveComponent.SetMaterial` (`self.Sphere`) 0 (`self.Spark Material`))
  (set `self.Starting World Location` (`SceneComponent.K2_GetComponentLocation` (`self.Sphere`))))

(event `self.Sphere1.OnComponentBeginOverlap`
  (params (OverlappedComponent :type "PrimitiveComponent Object Reference") (OtherActor :type "Actor Object Reference") (OtherComp :type "PrimitiveComponent Object Reference") (OtherBodyIndex :type Integer) (bFromSweep :type Boolean) (SweepResult :type "HitResult Structure (by ref)"))
  (bind _asbp_base_character (cast `/Game/Blueprints/Player_Blueprints/BP_BaseCharacter` OtherActor))
  (`/Game/Blueprints/Player_Blueprints/BP_BaseCharacter.Increase Spark Count` _asbp_base_character)
  (`KismetSystemLibrary.Delay` 0.01)
  (`self.K2_DestroyActor`)
  (`self.Unlock Mechanic` (`self.Unlock Double Jump?`) (`self.Unlock Climb?`) (`self.Unlock Grapple?`)))

(fn `Unlock Mechanic`
  (params (`Unlock Double Jump?` :type Boolean) (`Unlock Climb?` :type Boolean) (`Unlock Grapple?` :type Boolean))
  (bind _asbp_base_character (cast `/Game/Blueprints/Player_Blueprints/BP_BaseCharacter` (`GameplayStatics.GetPlayerPawn` 0)))
  (if `Unlock Grapple?`
    (set `/Game/Blueprints/Player_Blueprints/BP_BaseCharacter.Grapple Unlocked?` `Unlock Grapple?` _asbp_base_character))
  (if `Unlock Climb?`
    (set `/Game/Blueprints/Player_Blueprints/BP_BaseCharacter.Climb Unlocked?` `Unlock Climb?` _asbp_base_character))
  (if `Unlock Double Jump?`
    (`/Game/Blueprints/Player_Blueprints/BP_BaseCharacter.Increase Jump Count` _asbp_base_character)))

(fn `UserConstructionScript`)