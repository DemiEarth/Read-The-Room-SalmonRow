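; Player base character with movement, jumping, sprint, unlockable wall climbing and a grapple hook, plus a spark count shown in a HUD widget.
; Climbing uses Flying movement mode, with forward traces that attach the capsule, align it to surface normals and drop it off edges.
; The grapple shares the spark ability input, traces along the camera, animates a cable and launches the character, then cools down.
; Sparks scale jump height and grapple range.
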(event `EnhancedInput|/Game/Blueprints/Player_Blueprints/Controls/IA_Jump`
  (params (ActionValue :type Boolean) (ElapsedSeconds :type "Float (double-precision)") (TriggeredSeconds :type "Float (double-precision)") (InputAction :type "InputAction Object Reference" :default "/Game/Blueprints/Player_Blueprints/Controls/IA_Jump.IA_Jump"))
  ;[0.0137 1 0.9276 0.5 40] Jumping
  ;; Jump Bases
  (:`Triggered`
    (`self.Jump`))
  (:`Completed`
    (`self.StopJumping`)))

(event `EnhancedInput|/Game/Blueprints/Player_Blueprints/Controls/IA_SparkAbility`
  (params (ActionValue :type Boolean) (ElapsedSeconds :type "Float (double-precision)") (TriggeredSeconds :type "Float (double-precision)") (InputAction :type "InputAction Object Reference" :default "/Game/Blueprints/Player_Blueprints/Controls/IA_SparkAbility.IA_SparkAbility"))
  (bind _charactermovement (`self.CharacterMovement`))
  (bind _capsulecomponent (`self.CapsuleComponent`))
  ;[1 0.4983 0 0.5 40] Climbing
  ;; Start Climbing
  (:`Started`
    (if (and (`|EnumInequality` (`CharacterMovementComponent.MovementMode` (`self.CharacterMovement`)) "MOVE_Flying") (`self.Climb Unlocked?`))
      (bind (_outhit _returnvalue) (`self.Climbing Line Trace` (`self.Climb Distance`)))
      (if _returnvalue
        (`CharacterMovementComponent.SetMovementMode` _charactermovement "MOVE_Flying" 0)
        (set `CharacterMovementComponent.bOrientRotationToMovement` false _charactermovement)
        (bind (_bblockinghit _binitialoverlap _time _distance _location _impactpoint _normal) (`GameplayStatics.BreakHitResult` _outhit))
        (`KismetSystemLibrary.MoveComponentTo` _capsulecomponent (+ _location (* _normal (`CapsuleComponent.CapsuleRadius` _capsulecomponent))) (`KismetMathLibrary.MakeRotFromX` (* _normal -1.0)))))))

(event `EnhancedInput|/Game/Blueprints/Player_Blueprints/Controls/IA_Look`
  (params (ActionValue :type "Vector2D Structure") (ElapsedSeconds :type "Float (double-precision)") (TriggeredSeconds :type "Float (double-precision)") (InputAction :type "InputAction Object Reference" :default "/Game/Blueprints/Player_Blueprints/Controls/IA_Look.IA_Look"))
  ;[0.1377 1 0 0.5 40] Base Movement
  ;; Player Looking
  (:`Triggered`
    (`self.AddControllerYawInput` ActionValue_X)
    (`self.AddControllerPitchInput` ActionValue_Y)))

(event `EnhancedInput|/Game/Blueprints/Player_Blueprints/Controls/IA_Forward`
  (params (ActionValue :type "Float (double-precision)") (ElapsedSeconds :type "Float (double-precision)") (TriggeredSeconds :type "Float (double-precision)") (InputAction :type "InputAction Object Reference" :default "/Game/Blueprints/Player_Blueprints/Controls/IA_Forward.IA_Forward"))
  (bind (_returnvalue_roll _returnvalue_pitch _returnvalue_yaw) (`KismetMathLibrary.BreakRotator` (`self.GetControlRotation`)))
  ;[0.1377 1 0 0.5 40] Base Movement
  ;; Player Moving Forward & Back
  (:`Triggered`
    (switch `EMovementMode` (`CharacterMovementComponent.MovementMode` (`self.CharacterMovement`))
      (:`MOVE_Walking`
        (`self.AddMovementInput` (`KismetMathLibrary.GetForwardVector` (`KismetMathLibrary.MakeRotator` 0.0 0.0 _returnvalue_yaw)) ActionValue :!label _label))
      (:`MOVE_Falling`
        (goto _label))
      (:`MOVE_Flying`
        (`self.Climb Movement` (`self.GetActorUpVector`) ActionValue)))))

(event `Increase Jump Count`
  ;[0.0137 1 0.9276 0.5 40] Jumping
  ;; Increases Jump Count
  (set `self.JumpMaxCount` (`self.Jumps Possible`)))

(event `Increase Jump height`
  ;[0.0137 1 0.9276 0.5 40] Jumping
  ;; Increases Jump Height
  (set `CharacterMovementComponent.JumpZVelocity` (`KismetMathLibrary.Conv_IntToDouble` (+ (`self.Base Jump Value`) (* (`self.Sparks Count`) 35))) (`self.CharacterMovement`)))

(event `Climb Movement`
  (params (WorldDirection :type "Vector Structure") (ScaleValue :type "Float (single-precision)"))
  ;[1 0.4983 0 0.5 40] Climbing
  ;; Climb Movement
  (bind (_outhit _returnvalue) (`self.Climbing Line Trace` 120.0))
  (if _returnvalue
    (`self.AddMovementInput` WorldDirection ScaleValue)
    (bind (_direction _rotation) (`Timeline|Climb Align To Surface` :!via `PlayFromStart`)
      (:`Update`
        (`self.K2_SetActorRotation` (`KismetMathLibrary.RLerp` (`self.K2_GetActorRotation`) (`KismetMathLibrary.MakeRotFromX` (* (`.Normal` (`GameplayStatics.BreakHitResult` _outhit)) -1.0)) _rotation))))
    (else
      (`self.Stop Climbing`))))

(event `EnhancedInput|/Game/Blueprints/Player_Blueprints/Controls/IA_Right`
  (params (ActionValue :type "Float (double-precision)") (ElapsedSeconds :type "Float (double-precision)") (TriggeredSeconds :type "Float (double-precision)") (InputAction :type "InputAction Object Reference" :default "/Game/Blueprints/Player_Blueprints/Controls/IA_Right.IA_Right"))
  (bind (_returnvalue_roll _returnvalue_pitch _returnvalue_yaw) (`KismetMathLibrary.BreakRotator` (`self.GetControlRotation`)))
  ;[0.1377 1 0 0.5 40] Base Movement
  ;; Player Moving Right and Left
  (:`Triggered`
    (switch `EMovementMode` (`CharacterMovementComponent.MovementMode` (`self.CharacterMovement`))
      (:`MOVE_Walking`
        (`self.AddMovementInput` (`KismetMathLibrary.GetRightVector` (`KismetMathLibrary.MakeRotator` 0.0 0.0 _returnvalue_yaw)) ActionValue :!label _label_2))
      (:`MOVE_Falling`
        (goto _label_2))
      (:`MOVE_Flying`
        (`self.Climb Movement` (`self.GetActorRightVector`) ActionValue)))))

(event `Reset Jump Height`
  ;[0.0137 1 0.9276 0.5 40] Jumping
  ;; Reset Jump Value to Base
  (set `CharacterMovementComponent.JumpZVelocity` (`KismetMathLibrary.Conv_IntToDouble` (`self.Base Jump Value`)) (`self.CharacterMovement`)))

(event `Stop Climbing`
  (bind (_returnvalue_roll _returnvalue_pitch _returnvalue_yaw) (`KismetMathLibrary.BreakRotator` (`self.K2_GetActorRotation`)))
  (bind _charactermovement (`self.CharacterMovement`))
  ;[1 0.4983 0 0.5 40] Climbing
  ;; Stop Climbing
  (`CharacterMovementComponent.SetMovementMode` _charactermovement "MOVE_Falling" 0)
  (set `CharacterMovementComponent.bOrientRotationToMovement` true _charactermovement)
  (`KismetSystemLibrary.Delay` 0.2)
  (`self.K2_SetActorRotation` (`KismetMathLibrary.MakeRotator` 0.0 0.0 _returnvalue_yaw)))

(event `InputAction|Sprint`
  (params (Key :type "Key Structure"))
  (bind _charactermovement (`self.CharacterMovement`))
  ;[0.1377 1 0 0.5 40] Base Movement
  ;; Sprint - Needs Edit
  (:`Pressed`
    (set `CharacterMovementComponent.MaxWalkSpeed` 1000.0 _charactermovement))
  (:`Released`
    (set `CharacterMovementComponent.MaxWalkSpeed` 600.0 _charactermovement)))

(event `EnhancedInput|/Game/Blueprints/Player_Blueprints/Controls/IA_SparkAbility`
  (params (ActionValue :type Boolean) (ElapsedSeconds :type "Float (double-precision)") (TriggeredSeconds :type "Float (double-precision)") (InputAction :type "InputAction Object Reference" :default "/Game/Blueprints/Player_Blueprints/Controls/IA_SparkAbility.IA_SparkAbility"))
  (bind _returnvalue (`self.K2_GetActorLocation`))
  ;[0.9844 0 0.05376 0.5 40] Grapple
  ;; Grapple Action
  (:`Triggered`
    (if (and (`self.Can Grapple?`) (`self.Grapple Unlocked?`))
      (set `self.Can Grapple?` false)
      (set `self.Is Grappling?` true)
      (bind (_outhit _returnvalue_2) (`KismetSystemLibrary.LineTraceSingle` :`Start` _returnvalue :`End` (+ _returnvalue (* (`SceneComponent.GetForwardVector` (`self.Player Camera`)) (+ (`self.Base Grapple Distance`) (* (`self.Sparks Count`) 25)))) :`TraceChannel` "TraceTypeQuery1" :`DrawDebugType` "ForDuration"))
      (if _returnvalue_2
        (bind (_bblockinghit _binitialoverlap _time _distance _location) (`GameplayStatics.BreakHitResult` _outhit))
        (set `self.Grapple Location` _location)
        (`self.Shoot Grapple Hook`)
        (`self.LaunchCharacter` (0.0 0.0 500.0) true true)
        (`KismetSystemLibrary.Delay` 0.2)
        (`self.LaunchCharacter` (* (- _location _returnvalue) 2.5))
        (`KismetSystemLibrary.Delay` 0.5)
        (`self.Reset Grapple Hook`)
        (else
          (`self.Reset Grapple Hook`))))))

(event `Shoot Grapple Hook`
  (bind _grapplecable (`self.GrappleCable`))
  ;[0.9844 0 0.05376 0.5 40] Grapple
  ;; Shoot Grapple
  (`SceneComponent.SetVisibility` _grapplecable true false)
  (bind (_direction _interp_speed) (`Timeline|Grapple Timeline` :!via `PlayFromStart`)
    (:`Update`
      (`SceneComponent.K2_SetWorldLocation` _grapplecable (`KismetMathLibrary.VInterpTo` (`SceneComponent.K2_GetComponentLocation` _grapplecable) (`self.Grapple Location`) (`self.Delta Seconds (For Grapple)`) _interp_speed) false false))))

(event `self.ReceiveTick`
  (params (DeltaSeconds :type "Float (single-precision)"))
  ;[0.9844 0 0.05376 0.5 40] Grapple
  ;;[0 0 0 0.5] Fucking Change this shit is so bad
  (`|ExecutionSequence`
    (:`then_0`
      (set `self.Delta Seconds (For Grapple)` DeltaSeconds))))

(event `Reset Grapple Hook`
  ;[0.9844 0 0.05376 0.5 40] Grapple
  ;; Reset Grapple
  (`SceneComponent.SetVisibility` (`self.GrappleCable`) false false)
  (set `self.Is Grappling?` false)
  (`KismetSystemLibrary.Delay` (`self.Grapple Cooldown`))
  (set `self.Can Grapple?` true))

(event `Increase Spark Count`
  ;[0.15 0.15 0.15 0.5 40] sparks
  ;; Increases Spark Count and Deals with all Logic Tied to it
  (bind _output_get (set `self.Sparks Count` (+ (`self.Sparks Count`) 1)))
  (`/Game/Blueprints/Sparks/SparksUI/WB_SparksUI.Update Spark Count UI` (`self.Sparks UI Ref`) _output_get)
  (`self.Increase Jump height`))

(event `self.ReceiveBeginPlay`
  ;[0.15 0.15 0.15 0.5 40] sparks
  ;; Creates UI that Keeps Track of Sparks
  (bind _returnvalue (`|CreateWidget` "/Game/Blueprints/Sparks/SparksUI/WB_SparksUI.WB_SparksUI_C"))
  (bind _output_get (set `self.Sparks UI Ref` _returnvalue))
  (`UserWidget.AddToViewport` _output_get 0))

(event `Update Spark Count`
  ;[0.15 0.15 0.15 0.5 40] sparks
  (`/Game/Blueprints/Sparks/SparksUI/WB_SparksUI.Update Spark Count UI` (`self.Sparks UI Ref`) (`self.Sparks Count`)))

(fn `Climbing Line Trace`
  (params (`Attach Distance` :type "Float (double-precision)"))
  (returns (OutHit :type "HitResult Structure") (ReturnValue :type Boolean))
  (bind _returnvalue (`self.K2_GetActorLocation`))
  (bind (_outhit _returnvalue_2) (`KismetSystemLibrary.LineTraceSingle` _returnvalue (+ _returnvalue (* (`KismetMathLibrary.GetForwardVector` (`self.K2_GetActorRotation`)) `Attach Distance`)) "TraceTypeQuery1"))
  (return _outhit _returnvalue_2))

(fn `UserConstructionScript`)