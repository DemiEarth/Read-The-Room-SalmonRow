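; BP_Key_ is a level-progression pickup that advances a BP_BaseCharacter to the next level when touched.
; On BeginPlay it applies its configurable material to the Sphere component.
; The first character overlap with Sphere1 sets CurrentLevel to NextLevel, teleports the character to Spawn unless DoNotTP is set, and resets SparksCount.
; A DoOnce guards against repeat triggers, and the key destroys itself after a short delay.
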(event `self.ReceiveBeginPlay`
  (`PrimitiveComponent.SetMaterial` (`self.Sphere`) 0 (`self.Material`)))

(event `self.Sphere1.OnComponentBeginOverlap`
  (params (OverlappedComponent :type "PrimitiveComponent Object Reference") (OtherActor :type "Actor Object Reference") (OtherComp :type "PrimitiveComponent Object Reference") (OtherBodyIndex :type Integer) (bFromSweep :type Boolean) (SweepResult :type "HitResult Structure (by ref)"))
  (bind _asbp_base_character (cast `/Game/Blueprints/Player_Blueprints/BP_BaseCharacter` OtherActor))
  (`/Engine/EditorBlueprintResources/StandardMacros.DoOnce` false
    (:`Completed`
      (set `/Game/Blueprints/Player_Blueprints/BP_BaseCharacter.Current Level` (`self.Next Level`) _asbp_base_character)
      (if (not (`self.Do Not TP?`))
        (`self.K2_SetActorLocation` _asbp_base_character (`self.Spawn`) false false))
      (set `/Game/Blueprints/Player_Blueprints/BP_BaseCharacter.Sparks Count` 0 _asbp_base_character)
      (`KismetSystemLibrary.Delay` 0.1)
      (`self.K2_DestroyActor`))))

(fn `UserConstructionScript`)