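; Portal actor that pairs with a linked portal, using scene captures and render targets to display a view through each.
; On construction, an enabled primary links its partner back and assigns both render targets and face materials.
; While enabled, Tick resizes its target to the viewport and positions the partner's capture using the relative transform between Backfacing and the player camera.
; UpdateSceneCapture is empty; its older mirrored-camera math is disconnected.
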(event `self.ReceiveBeginPlay`
  (bind _asbp_base_character (cast `/Game/Blueprints/Player_Blueprints/BP_BaseCharacter` (`GameplayStatics.GetPlayerCharacter` 0)))
  (set `self.Player Reference` _asbp_base_character))

(event `self.ReceiveTick`
  (params (DeltaSeconds :type "Float (single-precision)"))
  (`self.UpdateSceneCapture`)
  (if (`self.Is Enabled?`)
    (`self.Update Render Target`)))

(fn `Primary Setup`
  (bind _linked_portal (`self.Linked Portal`))
  (if (and (`self.Is Enabled?`) (`self.Is Primary?`))
    (`self.Setup Render Target` (`self.Primary Portal Render Target`))
    (set `/Game/Blueprints/Portals/BP_Portal1.Linked Portal` self _linked_portal)
    (`self.Setup Render Target` _linked_portal (`self.Secondary Portal Render Target`))
    (else
      (`KismetSystemLibrary.PrintString` "Hello"))))

(fn `Setup Render Target`
  (params (`Render Target` :type "TextureRenderTarget2D Object Reference"))
  (set `SceneCaptureComponent2D.TextureTarget` `Render Target` (`self.SceneCaptureComponent2D`))
  (`PrimitiveComponent.SetMaterial` (`self.Portal Face`) 0 (select `bool` (`self.Is Primary?`) :`false` (`self.First Portals`) :`true` (`self.Second Portal`))))

(fn `Update Render Target`
  (bind (_returnvalue_x _returnvalue_y) (`KismetMathLibrary.BreakVector2D` (`WidgetLayoutLibrary.GetViewportSize`)))
  (bind (_returnvalue_location _returnvalue_rotation) (`KismetMathLibrary.BreakTransform` (`KismetMathLibrary.MakeRelativeTransform` (`SceneComponent.K2_GetComponentToWorld` (`self.Backfacing`)) (`SceneComponent.K2_GetComponentToWorld` (`/Game/Blueprints/Player_Blueprints/BP_BaseCharacter.Player Camera` (`self.Player Reference`))))))
  (`KismetRenderingLibrary.ResizeRenderTarget2D` (`SceneCaptureComponent2D.TextureTarget` (`self.SceneCaptureComponent2D`)) (`KismetMathLibrary.FTrunc` _returnvalue_x) (`KismetMathLibrary.FTrunc` _returnvalue_y))
  (`SceneComponent.K2_SetRelativeLocationAndRotation` (`/Game/Blueprints/Portals/BP_Portal1.SceneCaptureComponent2D` (`self.Linked Portal`)) _returnvalue_location _returnvalue_rotation false false))

(fn `UpdateSceneCapture`)

(fn `UserConstructionScript`
  (`self.Primary Setup`))